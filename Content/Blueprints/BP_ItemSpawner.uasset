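; Item spawner actor that places a fire-rate pickup at a random spot inside its SpawnVolume box.
; The custom SpawnItem event checks that the TwinStickMode game mode is no longer waiting to start, then waits a random delay before spawning one BP_FireRateItem.
; The event does not re-trigger itself, and nothing in this Blueprint calls it, as BeginPlay and Tick are unused.
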(event Custom|SpawnItem
  (bind _spawnvolume (Variables|Default|GetSpawnVolume))
  ;[1 1 1] Spawnaa itemeitö kun peli pyörii satunnaisilla viiveillä väliltä 5-14s
  (bind _astwin_stick_mode (Utilities|Casting|CastToTwinStickMode (Game|GetGameMode)))
  (if (not (Variables|/Game/Blueprints/TwinStickMode.TwinStickMode_C|GetWaitingToStart _astwin_stick_mode))
    (Utilities|FlowControl|Delay (Math|Random|RandomFloatinRange 5.0 14.0))
    (Game|SpawnActorfromClass "/Game/Blueprints/BP_FireRateItem.BP_FireRateItem_C" (Math|Transform|MakeTransform (Math|Random|RandomPointinBoundingBox (Transformation|GetWorldLocation _spawnvolume) (Components|Box|GetScaledBoxExtent _spawnvolume)) "0, 0, 0" "1.000000,1.000000,1.000000") "Undefined" "MultiplyWithRoot" 0 0)))

(event EventBeginPlay)

(event Collision|EventActorBeginOverlap
  (params (OtherActor :type Actor%20Object%20Reference)))

(event EventTick
  (params (DeltaSeconds :type Float%20%28single-precision%29)))

(fn ConstructionScript)