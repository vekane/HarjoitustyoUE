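; EnemyCharacter is a twin-stick shooter enemy that damages the hero on contact and awards score when killed.
; Overlapping a HeroCharacter starts a looping DamageHero timer, which is cleared when that hero leaves.
; AffectHealth prints health and, on death, updates TwinStickMode score and kill count, disables pawn collision, detaches the controller, then explodes after a delay.
; The construction script tints the mesh through a dynamic material instance.
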(event Custom|DamageHero
  ;[1 1 1] Määritä aiheutettu vahinko pelaajalle
  (Default|AffectHealth (Variables|Default|GetHero) (Variables|Default|GetDamage)))

(event EventBeginPlay)

(event Collision|EventActorBeginOverlap
  (params (OtherActor :type Actor%20Object%20Reference))
  ;[1 1 1] Aiheuta pelaajalle vahinkoa jos osuu viholliseen
  (bind _ashero_character (Utilities|Casting|CastToHeroCharacter OtherActor))
  (Variables|Default|SetHero _ashero_character)
  (Utilities|Time|SetTimerbyFunctionName 0 "DamageHero" 0.5 true))

(event EventTick
  (params (DeltaSeconds :type Float%20%28single-precision%29)))

(event EventAffectHealth
  (params (Delta :type Float%20%28double-precision%29))
  (bind _capsulecomponent (Variables|Default|GetCapsuleComponent))
  ;[1 1 1] Laske healthin määrä ja tarkista onko kuolema tosi
  (Class|BaseCharacter|CalculateHealth Delta)
  (Development|PrintString (Utilities|String|ToString(Float) (Variables|Default|GetHealth)) false)
  (if (Variables|Default|GetisDead)
    ;[1 1 1] Kuoleman jälkeen nosta pelaajan scorea ja nosta tapettujen vihollisten määrää
    (bind _astwin_stick_mode (Utilities|Casting|CastToTwinStickMode (Game|GetGameMode)))
    (Default|IncrementScore _astwin_stick_mode (Variables|Default|GetScore))
    (Default|IncrementEnemiesDied _astwin_stick_mode)
    ;[1 1 1] Muuta collisionia ettei se reagoi pelaajan kanssa
    (Collision|SetCollisionResponsetoChannel _capsulecomponent "ECC_WorldDynamic" "ECR_Ignore")
    (Collision|SetCollisionResponsetoChannel _capsulecomponent "ECC_Pawn" "ECR_Ignore")
    (Class|Pawn|DetachfromControllerPendingDestroy)
    ;[1 1 1] Delayn jälkeen räjähdysefekti ja actorin poistaminen
    (Utilities|FlowControl|Delay 3.0)
    (Game|SpawnActorfromClass "/Game/Blueprints/Explosion.Explosion_C" (Transformation|GetActorTransform) "Undefined" "MultiplyWithRoot" 0 0)
    (Actor|DestroyActor)))

(event Collision|EventActorEndOverlap
  (params (OtherActor :type Actor%20Object%20Reference))
  ;[1 1 1] Resettaa DamageHero funktion timer
  (if (== OtherActor (Variables|Default|GetHero))
    (Utilities|Time|ClearTimerbyFunctionName 0 "DamageHero")))

(fn ConstructionScript
  (bind _returnvalue (Rendering|Material|CreateDynamicMaterialInstance (Variables|Character|GetMesh) 0 0 "None" :!class /Script/Engine.PrimitiveComponent))
  (bind _output_get (Variables|Default|SetDynaMat _returnvalue))
  (Rendering|Material|SetVectorParameterValue _output_get "BodyColor" (Variables|Default|GetEenemyColor) :!class /Script/Engine.MaterialInstanceDynamic))