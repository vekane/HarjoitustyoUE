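; Enemy spawner actor for a twin-stick shooter that adds EnemyCharacter AI pawns at random points inside its SpawnVolume box.
; SpawnEnemy does nothing while the TwinStickMode game mode is waiting to start, and otherwise spawns one enemy if the level's EnemyCharacter count is below MaxEnemies.
; IncrementEnemies raises that cap by a fixed step.
; Nothing in this graph calls either event, and BeginPlay and Tick are unused.
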(event Custom|SpawnEnemy
  (bind _spawnvolume (Variables|Default|GetSpawnVolume))
  ;[0 1 0.4414] Enemy spawner
  (bind _astwin_stick_mode (Utilities|Casting|CastToTwinStickMode (Game|GetGameMode)))
  (if (not (Variables|/Game/Blueprints/TwinStickMode.TwinStickMode_C|GetWaitingToStart _astwin_stick_mode))
    (bind _outactors (Actor|GetAllActorsOfClass "/Game/Blueprints/EnemyCharacter.EnemyCharacter_C"))
    (if (< (Utilities|Array|Length _outactors) (Variables|Default|GetMaxEnemies))
      (AI|SpawnAIFromClass "/Game/Blueprints/EnemyCharacter.EnemyCharacter_C" 0 (Math|Random|RandomPointinBoundingBox (Transformation|GetWorldLocation _spawnvolume) (Components|Box|GetScaledBoxExtent _spawnvolume)) "0, 0, 0" false 0))))

(event Custom|IncrementEnemies
  ;[0 1 0.2461] Nosta vihollisten lukumäärää
  (Variables|Default|SetMaxEnemies (+ (Variables|Default|GetMaxEnemies) 5)))

(event EventBeginPlay)

(event Collision|EventActorBeginOverlap
  (params (OtherActor :type Actor%20Object%20Reference)))

(event EventTick
  (params (DeltaSeconds :type Float%20%28single-precision%29)))

(fn ConstructionScript)